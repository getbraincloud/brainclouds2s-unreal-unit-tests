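; Base Blueprint for S2S tests that sets up and services a server-to-server context.
; PrepareTest loads test credentials, creates an auto-authenticating S2S context from them, stores it and enables its logging.
; Tick pumps the context's callbacks each frame while it is valid.
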(event EventTick
  (params (DeltaSeconds :type Float%20%28single-precision%29))
  (bind _s2s (Variables|Default|GetS2S))
  (Utilities|IsValid _s2s
    (:Is%20Valid
      (Class|BrainCloudS2S|RunCallbacks _s2s))))

(event EventPrepareTest
  (CallFunction|PrepareTest))

(fn ConstructionScript)

(fn PrepareTest
  (bind _returnvalue (Class|S2SBlueprintTestLibrary|LoadS2STestCredentials))
  (bind _returnvalue_2 (Class|BrainCloudS2S|CreateS2SContext (.AppId (Utilities|Struct|BreakS2STestCredentials _returnvalue)) (.ServerName (Utilities|Struct|BreakS2STestCredentials _returnvalue)) (.ServerSecret (Utilities|Struct|BreakS2STestCredentials _returnvalue)) (.Url (Utilities|Struct|BreakS2STestCredentials _returnvalue)) true))
  (bind _output_get (Variables|Default|SetS2S _returnvalue_2))
  (Class|BrainCloudS2S|S2SSetLogEnabled _output_get true))