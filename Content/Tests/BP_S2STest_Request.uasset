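; Functional test actor that checks a server-to-server (S2S) request to the globalFileV3 service.
; On test start it sends a hard-coded JSON payload requesting a recursive global file list from the root folder.
; The response callback passes the JSON and test context to ReportResult, then finishes the test as succeeded or failed on that result, without reading the Success flag.
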(event Custom|OnResponse
  (params (bSuccess :type Boolean) (JsonResponse :type String))
  (bind _returnvalue (Class|S2SBlueprintTestLibrary|ReportResult JsonResponse (Variables|Default|GetTestContext)))
  (if _returnvalue
    (Class|FunctionalTest|FinishTest "Succeeded")
    (else
      (Class|FunctionalTest|FinishTest "Failed"))))

(event EventStartTest
  (Class|BrainCloudS2S|S2SRequest (Variables|Default|GetS2S) "{\"service\":\"globalFileV3\",\"operation\":\"SYS_GET_GLOBAL_FILE_LIST\",\"data\":{\"folderPath\":\"\",\"recurse\":true}}" (delegate Custom|OnResponse)))

(event EventTick
  (params (DeltaSeconds :type Float%20%28single-precision%29))
  (|CallParentFunction DeltaSeconds) ; This node is disabled and will not be called.\nDrag off pins to build functionality.
)

(fn ConstructionScript
  (|CallParentFunction))