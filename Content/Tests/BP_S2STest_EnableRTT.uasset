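; Functional test Blueprint that checks whether the brainCloud-style S2S client can enable its RTT real-time connection.
; On test start it calls S2SEnableRTT on the S2S RTT comms object with success and failure callbacks.
; The success callback reports the result and finishes the test as succeeded.
; The failure callback is empty, and a Failed finish node is left unconnected.
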(event Custom|OnRTTDisconnected
  (params (bSuccess :type Boolean) (JsonResponse :type String)))

(event Custom|OnRTTEnabled
  (params (bSuccess :type Boolean) (JsonResponse :type String))
  (Class|S2SBlueprintTestLibrary|ReportResultSimple bSuccess "" (Variables|Default|GetTestContext))
  (Class|FunctionalTest|FinishTest "Succeeded" "[SUCCESS] RTT Connected successfully "))

(event EventStartTest
  (Class|S2SRTTComms|S2SEnableRTT (Class|BrainCloudS2S|GetRTTComms (Variables|Default|GetS2S)) (delegate Custom|OnRTTEnabled) (delegate Custom|OnRTTDisconnected)))

(event EventTick
  (params (DeltaSeconds :type Float%20%28single-precision%29))
  (|CallParentFunction DeltaSeconds) ; This node is disabled and will not be called.\nDrag off pins to build functionality.
)

(fn ConstructionScript
  (|CallParentFunction))