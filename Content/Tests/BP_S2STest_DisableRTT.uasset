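; Test Blueprint that checks the S2S client can enable and then disable its RTT (real-time) connection.
; StartTest requests RTT through the S2S RTT comms object with success and failure callbacks.
; On success it reports the result, calls disable, and passes immediately without waiting for disconnect confirmation.
; The failure callback reports a failed connection or abrupt disconnect and fails the test.
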(event Custom|OnRTTEnabled
  (params (bSuccess :type Boolean) (JsonResponse :type String))
  (Class|S2SBlueprintTestLibrary|ReportResultSimple bSuccess "" (Variables|Default|GetTestContext))
  (Class|S2SRTTComms|S2SDisableRTT (Class|BrainCloudS2S|GetRTTComms (Variables|Default|GetS2S)))
  (Class|S2SBlueprintTestLibrary|ReportResultSimple true "Disabled and disconnected from RTT" (Variables|Default|GetTestContext))
  (Class|FunctionalTest|FinishTest "Succeeded"))

(event Custom|OnRTTDisconnected
  (params (bSuccess :type Boolean) (JsonResponse :type String))
  (Class|S2SBlueprintTestLibrary|ReportResultSimple false "RTT Failed to connect or disconnected abruptly" (Variables|Default|GetTestContext))
  (Class|FunctionalTest|FinishTest "Failed" "RTT Failed to connect or disconnected abruptly"))

(event EventStartTest
  (Class|S2SRTTComms|S2SEnableRTT (Class|BrainCloudS2S|GetRTTComms (Variables|Default|GetS2S)) (delegate Custom|OnRTTEnabled) (delegate Custom|OnRTTDisconnected)))

(event EventTick
  (params (DeltaSeconds :type Float%20%28single-precision%29))
  (|CallParentFunction DeltaSeconds) ; This node is disabled and will not be called.\nDrag off pins to build functionality.
)

(fn ConstructionScript
  (|CallParentFunction))