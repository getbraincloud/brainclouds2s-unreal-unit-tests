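; Functional test that verifies an S2S client receives a chat message over RTT (real-time connection).
; StartTest registers an RTT callback and enables RTT, then sends S2S JSON requests to join the app's system channel and post a message.
; The callback passes when it parses an incoming chat event.
; A failed channel join, or an RTT disconnect while RTTSuccess is false, fails the test.
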(event Custom|OnRTTCallback
  (params (bSuccess :type Boolean) (JsonResponse :type String))
  (bind _receivedmessage (CallFunction|CheckifReceivedChatMessage JsonResponse))
  (if _receivedmessage
    (Class|FunctionalTest|FinishTest "Succeeded" "[SUCCESS] RTT Message received")))

(event Custom|OnRTTEnabled
  (params (bSuccess :type Boolean) (JsonResponse :type String))
  (Class|S2SBlueprintTestLibrary|ReportResultSimple bSuccess JsonResponse (Variables|Default|GetTestContext))
  (Class|BrainCloudS2S|S2SRequest (Variables|Default|GetS2S) (Utilities|String|Append "{\"service\":\"chat\",\"operation\":\"SYS_CHANNEL_CONNECT\",\"data\":{\"channelId\":\"" (CallFunction|GetSysChannelId) "\",\"maxReturn\":0}}") (delegate Custom|OnJoinChannelResponse)))

(event Custom|OnRTTDisconnected
  (params (bSuccess :type Boolean) (JsonResponse :type String))
  (if (not (Variables|Default|GetRTTSuccess))
    (Class|FunctionalTest|FinishTest "Failed" "[SUCCESS] RTT Disconnected abruptly")))

(event Custom|OnJoinChannelResponse
  (params (bSuccess :type Boolean) (JsonResponse :type String))
  (bind _returnvalue (Class|S2SBlueprintTestLibrary|ReportResult JsonResponse (Variables|Default|GetTestContext)))
  (if _returnvalue
    (Class|BrainCloudS2S|S2SRequest (Variables|Default|GetS2S) (Utilities|String|Append "{\"service\":\"chat\",\"operation\":\"SYS_POST_CHAT_MESSAGE\",\"data\":{\"channelId\":\"" (CallFunction|GetSysChannelId) "\",\"content\":{\"foo\":\"bar\",\"someData\":\"12345\"},\"recordInHistory\":false}}") (delegate Custom|OnPostMessageResponse))
    (else
      (Class|FunctionalTest|FinishTest "Failed" "Failed to join sys channel"))))

(event Custom|OnPostMessageResponse
  (params (bSuccess :type Boolean) (JsonResponse :type String))
  (Class|S2SBlueprintTestLibrary|ReportResult JsonResponse (Variables|Default|GetTestContext)))

(event EventStartTest
  (bind _s2s (Variables|Default|GetS2S))
  (bind _returnvalue (Class|BrainCloudS2S|GetRTTComms _s2s))
  (Class|S2SRTTComms|S2SRegisterRTTCallback _returnvalue (delegate Custom|OnRTTCallback))
  (Class|S2SRTTComms|S2SEnableRTT _returnvalue (delegate Custom|OnRTTEnabled) (delegate Custom|OnRTTDisconnected)))

(event EventTick
  (params (DeltaSeconds :type Float%20%28single-precision%29))
  (|CallParentFunction DeltaSeconds) ; This node is disabled and will not be called.\nDrag off pins to build functionality.
)

(fn ConstructionScript
  (|CallParentFunction))

(fn GetSysChannelId
  (bind _returnvalue (Class|S2SBlueprintTestLibrary|LoadS2STestCredentials))
  (return (Utilities|String|Append (Utilities|Struct|BreakS2STestCredentials _returnvalue) ":sy:mysyschannel")))

(fn CheckifReceivedChatMessage
  (params (jsonRTTMessage :type String))
  (bind (_outjsonobject _returnvalue) (Class|JsonBlueprintFunctionLibrary|FromString jsonRTTMessage))
  (bind (_outvalue _returnvalue_2) (|GetJsonField _outjsonobject "service"))
  (bind (_outvalue_2 _returnvalue_3) (|GetJsonField _outjsonobject "operation"))
  (if (Math|Boolean|ANDBoolean _returnvalue_2 _returnvalue _returnvalue_3 (Utilities|Enum|Equal(Enum) _outvalue "chat") (Utilities|Enum|Equal(Enum) _outvalue_2 "INCOMING"))
    (return true)
    (else
      (return false))))