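; Functional test that checks a server-to-server (S2S) RTT connection delivers a message to a registered callback.
; On start it registers the RTT callback, then enables RTT, whose success response is only reported.
; The first callback finishes the test as succeeded and sets a flag.
; The enable-failure handler fails the test unless that flag is set, though its message is labeled "[SUCCESS]".
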(event Custom|OnRTTCallback
  (params (bSuccess :type Boolean) (JsonResponse :type String))
  (Class|S2SBlueprintTestLibrary|ReportResultSimple true JsonResponse (Variables|Default|GetTestContext))
  (Variables|Default|SetRTTSuccess true)
  (Class|FunctionalTest|FinishTest "Succeeded" "[SUCCESS] RTT Callback received"))

(event Custom|OnRTTDisconnected
  (params (bSuccess :type Boolean) (JsonResponse :type String))
  (if (not (Variables|Default|GetRTTSuccess))
    (Class|FunctionalTest|FinishTest "Failed" "[SUCCESS] RTT Disconnected abruptly")))

(event Custom|OnRTTEnabled
  (params (bSuccess :type Boolean) (JsonResponse :type String))
  (Class|S2SBlueprintTestLibrary|ReportResultSimple bSuccess JsonResponse (Variables|Default|GetTestContext)))

(event EventStartTest
  (bind _s2s (Variables|Default|GetS2S))
  (bind _returnvalue (Class|BrainCloudS2S|GetRTTComms _s2s))
  (Class|S2SRTTComms|S2SRegisterRTTCallback _returnvalue (delegate Custom|OnRTTCallback))
  (Class|S2SRTTComms|S2SEnableRTT _returnvalue (delegate Custom|OnRTTEnabled) (delegate Custom|OnRTTDisconnected)))

(event EventTick
  (params (DeltaSeconds :type Float%20%28single-precision%29))
  (|CallParentFunction DeltaSeconds) ; This node is disabled and will not be called.\nDrag off pins to build functionality.
)

(fn ConstructionScript
  (|CallParentFunction))